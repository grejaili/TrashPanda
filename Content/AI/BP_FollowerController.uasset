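; AI controller for a follower pawn that prepares and starts its follow behavior.
; On BeginPlay it loads BB_Follower and stores the pawn's starting location as home and the first TopDownCharacter found as the follow target.
; It sets following as active but the follow-target flag off, then runs BT_FollowTarget, leaving all movement and decision logic to that behavior tree.
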(event EventBeginPlay
  (Class|AIController|UseBlackboard "/Game/AI/BB_Follower.BB_Follower")
  (AI|Components|Blackboard|SetValueasVector (AI|GetBlackboard self) (Variables|Default|GetHomeLocationKey) (Transformation|GetActorLocation (Pawn|GetControlledPawn)))
  (bind _outactors (Actor|GetAllActorsOfClass "/Game/TopDownBP/Blueprints/TopDownCharacter.TopDownCharacter_C"))
  (AI|Components|Blackboard|SetValueasObject (AI|GetBlackboard self) (Variables|Default|GetTargetToFollowKey) (Utilities|Array|Get(acopy) _outactors))
  (AI|Components|Blackboard|SetValueasBool (AI|GetBlackboard self) (Variables|Default|GetFollowTargetKey) false)
  (AI|Components|Blackboard|SetValueasBool (AI|GetBlackboard self) (Variables|Default|GetIsFollowingActiveKey) true)
  (AI|RunBehaviorTree "/Game/AI/BT_FollowTarget.BT_FollowTarget"))

(fn ConstructionScript)